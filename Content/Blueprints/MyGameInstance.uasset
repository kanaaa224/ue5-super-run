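; Game instance that holds the run state (area, score, lives, coins) and provides game flow functions.
; Functions reset and update that state, check for zero lives, and open the main and Gameover levels.
; Others show loading, tutorial and HUD widgets, though RemoveHUD removes a newly created widget rather than the displayed one.
; Init and Shutdown are empty, and GameOver's widget code is disconnected.
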(event EventInit)

(event EventShutdown)

(fn Loading
  (bind _returnvalue (UserInterface|CreateWidget "/Game/Blueprints/widget_loading.widget_loading_C"))
  (UserInterface|Viewport|AddtoViewport _returnvalue 0))

(fn GameInit
  (Variables|Default|SetCurrentArea 0)
  (Variables|Default|SetScore 0)
  (Variables|Default|SetLife 3)
  (Variables|Default|SetCoin 0))

(fn GameStart
  (Game|OpenLevel(byName) "gamemain"))

(fn GameTutorial
  (bind _returnvalue (UserInterface|CreateWidget "/Game/Blueprints/widget_tutorial.widget_tutorial_C"))
  (UserInterface|Viewport|AddtoViewport _returnvalue 0))

(fn GameOver
  (Game|OpenLevel(byObjectReference) "/Game/Maps/gameover.gameover"))

(fn AddScore
  (params (point :type Integer))
  (Variables|Default|SetScore (+ point (Variables|Default|GetScore))))

(fn AddCoin
  (params (coin :type Integer))
  (Variables|Default|SetCoin (+ coin (Variables|Default|GetCoin))))

(fn ReduceLife
  (Variables|Default|SetLife (- (Variables|Default|GetLife) 1)))

(fn CheckGameover
  (return (<= (Variables|Default|GetLife) 0)))

(fn AddHUD
  (bind _returnvalue (UserInterface|CreateWidget "/Game/Blueprints/widget_hud.widget_hud_C"))
  (UserInterface|Viewport|AddtoViewport _returnvalue 0))

(fn RemoveHUD
  (bind _returnvalue (UserInterface|CreateWidget "/Game/Blueprints/widget_hud.widget_hud_C"))
  (Widget|RemovefromParent _returnvalue))