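; Coin pickup actor that spins in the level and awards a coin and score when collected.
; Tick adds a fixed yaw step each frame, so spin speed depends on frame rate.
; When BP_ThirdPersonCharacter overlaps the Box, it spawns an effect at the coin, destroys itself and plays a sound at world origin.
; It then adds one coin and its Point value as score through MyGameInstance.
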(event OnComponentBeginOverlap(Box)
  (params (OverlappedComponent :type Primitive%20Component%20Object%20Reference) (OtherActor :type Actor%20Object%20Reference) (OtherComp :type Primitive%20Component%20Object%20Reference) (OtherBodyIndex :type Integer) (bFromSweep :type Boolean) (SweepResult :type Hit%20Result%20Structure%20%28by%20ref%29))
  (bind _returnvalue (Game|GetGameInstance))
  (bind _asmy_game_instance (Utilities|Casting|CastToMyGameInstance _returnvalue))
  (Utilities|Casting|CastToBP_ThirdPersonCharacter OtherActor)
  (Niagara|SpawnSystematLocation 0 (Transformation|GetActorLocation))
  (Actor|DestroyActor)
  (Audio|PlaySoundatLocation "/Game/Audio/se_itemget1.se_itemget1" "0, 0, 0" "0, 0, 0" 1.0 1.0 0.0 0 0 0 0)
  (Default|AddCoin _asmy_game_instance 1)
  (Default|AddScore _asmy_game_instance (Variables|Default|Getpoint)))

(event EventBeginPlay)

(event EventTick
  (params (DeltaSeconds :type Float%20%28single-precision%29))
  (bind _returnvalue (Transformation|GetActorRotation))
  (if (>= (.yaw _returnvalue) 3.6e+02)
    (Transformation|SetActorRotation (Math|Rotator|MakeRotator (.roll _returnvalue) (.pitch _returnvalue) 0.0))
    (else
      (Transformation|SetActorRotation (Math|Rotator|MakeRotator (.roll _returnvalue) (.pitch _returnvalue) (+ (.yaw _returnvalue) 1.0))))))

(fn ConstructionScript)