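; Fire block stage object that either hurts the player or is collected for points, depending on the player's Ability.
; On box overlap with the third-person character, it reads Ability from player 0's character.
; An Ability of 0 reduces life through MyGameInstance and plays a damage sound.
; Any other value destroys the block, plays an item-get sound and adds its Point value to the score.
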(event OnComponentBeginOverlap(Box)
  (params (OverlappedComponent :type Primitive%20Component%20Object%20Reference) (OtherActor :type Actor%20Object%20Reference) (OtherComp :type Primitive%20Component%20Object%20Reference) (OtherBodyIndex :type Integer) (bFromSweep :type Boolean) (SweepResult :type Hit%20Result%20Structure%20%28by%20ref%29))
  (Utilities|Casting|CastToBP_ThirdPersonCharacter OtherActor)
  (if (== (Variables|/Game/ThirdPerson/Blueprints/BP_ThirdPersonCharacter.BP_ThirdPersonCharacter_C|GetAbility (.AsBP%20Third%20Person%20Character (Utilities|Casting|CastToBP_ThirdPersonCharacter (Game|GetPlayerCharacter 0)))) 0)
    (Default|ReduceLife (.AsBP%20Game%20Instance (Utilities|Casting|CastToMyGameInstance (Game|GetGameInstance))))
    (Audio|PlaySoundatLocation "/Game/Audio/se_damage.se_damage" "0, 0, 0" "0, 0, 0" 1.0 1.0 0.0 0 0 0 0)
    (else
      (Actor|DestroyActor)
      (Audio|PlaySoundatLocation "/Game/Audio/se_itemget2.se_itemget2" "0, 0, 0" "0, 0, 0" 1.0 1.0 0.0 0 0 0 0)
      (Default|AddScore (.AsBP%20Game%20Instance (Utilities|Casting|CastToMyGameInstance (Game|GetGameInstance))) (Variables|Default|Getpoint)))))

(event EventBeginPlay)

(event Collision|EventActorBeginOverlap
  (params (OtherActor :type Actor%20Object%20Reference)))

(event EventTick
  (params (DeltaSeconds :type Float%20%28single-precision%29)))

(fn ConstructionScript)